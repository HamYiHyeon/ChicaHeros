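; Base grabbable tooth puzzle piece that snaps to other pieces to build an assembly.
; While overlapping, Tick attaches it to a lower-ID piece if signed rotation differences stay under a threshold, passing its piece list on and disabling its sphere.
; Grabbing follows RootActor links to the root, then reparents that root's listed pieces to the held one without collision.
; Dropping restores their collision.
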(event `self.ReceiveBeginPlay`
  ; BeginPlay
  (`KismetArrayLibrary.Array_Add` (`self.AttachedPieceArray`) self)
  (set `self.RootActor` self))

(event `self.Sphere.OnComponentBeginOverlap`
  (params (OverlappedComponent :type "PrimitiveComponent Object Reference") (OtherActor :type "Actor Object Reference") (OtherComp :type "PrimitiveComponent Object Reference") (OtherBodyIndex :type Integer) (bFromSweep :type Boolean) (SweepResult :type "HitResult Structure (by ref)"))
  ; AttachComponentToComponent
  (set `self.bOverlapping` true))

(event `self.Sphere.OnComponentEndOverlap`
  (params (OverlappedComponent :type "PrimitiveComponent Object Reference") (OtherActor :type "Actor Object Reference") (OtherComp :type "PrimitiveComponent Object Reference") (OtherBodyIndex :type Integer))
  ; AttachComponentToComponent
  (set `self.bOverlapping` false))

(event `self.ReceiveTick`
  (params (DeltaSeconds :type "Float (single-precision)"))
  ; AttachComponentToComponent
  (if (`self.bOverlapping`)
    (bind _asbp_tooth_piece_base (cast `/Game/BluePrints/PuzzleLevel/Tooth/BP_ToothPieceBase` (stale `self.Sphere.OnComponentBeginOverlap` OtherActor)))
    (if (and (> (`self.PieceID`) (`/Game/BluePrints/PuzzleLevel/Tooth/BP_ToothPieceBase.PieceID` _asbp_tooth_piece_base)) (<= (- (.roll (`self.K2_GetActorRotation` _asbp_tooth_piece_base)) (.roll (`self.K2_GetActorRotation`))) 20.0) (<= (- (.pitch (`self.K2_GetActorRotation` _asbp_tooth_piece_base)) (.pitch (`self.K2_GetActorRotation`))) 20.0) (<= (- (.yaw (`self.K2_GetActorRotation` _asbp_tooth_piece_base)) (.yaw (`self.K2_GetActorRotation`))) 20.0))
      (`SceneComponent.K2_AttachToComponent` (`self.ToothCell`) (`/Game/BluePrints/PuzzleLevel/Tooth/BP_ToothPieceBase.ToothCell` _asbp_tooth_piece_base) "None" "SnapToTarget" "SnapToTarget" "KeepWorld" true)
      (`PrimitiveComponent.SetCollisionEnabled` (`self.Sphere`) "NoCollision")
      (for _array_element (`self.AttachedPieceArray`)
        (`KismetArrayLibrary.Array_AddUnique` (`/Game/BluePrints/PuzzleLevel/Tooth/BP_ToothPieceBase.AttachedPieceArray` _asbp_tooth_piece_base) _array_element))
      (set `self.RootActor` _asbp_tooth_piece_base)
      (`KismetSystemLibrary.PrintString` (`KismetStringLibrary.Concat_StrStr` "Attach: " (`KismetSystemLibrary.GetDisplayName` _asbp_tooth_piece_base)))
      (set `self.bOverlapping` false))))

(event `self.GrabComponent.OnGrabbed`
  (bind _rootactor (`self.RootActor`))
  (bind _rootactor_2 (`/Game/BluePrints/PuzzleLevel/Tooth/BP_ToothPieceBase.RootActor` _rootactor))
  ; OnGrabbed
  (`KismetSystemLibrary.PrintString` (`KismetStringLibrary.Concat_StrStr` "grabbed: " (`KismetSystemLibrary.GetDisplayName` self)))
  (while (!= _rootactor_2 _rootactor)
    (bind _output_get (set `self.RootActor` _rootactor_2)))
  (`KismetSystemLibrary.PrintString` (`KismetStringLibrary.Concat_StrStr` "RootActor: " (`KismetSystemLibrary.GetDisplayName` _output_get)))
  (for _array_element (`/Game/BluePrints/PuzzleLevel/Tooth/BP_ToothPieceBase.AttachedPieceArray` _output_get)
    (bind _toothcell (`/Game/BluePrints/PuzzleLevel/Tooth/BP_ToothPieceBase.ToothCell` _array_element))
    (`KismetSystemLibrary.PrintString` (`KismetStringLibrary.Concat_StrStr` "Reattach: " (`KismetSystemLibrary.GetDisplayName` _toothcell)))
    (if (!= _array_element self)
      (`SceneComponent.K2_AttachToComponent` _toothcell (`self.ToothCell`) "None" "SnapToTarget" "SnapToTarget" "KeepWorld" true)
      (`PrimitiveComponent.SetCollisionEnabled` _toothcell "NoCollision")
      (`KismetSystemLibrary.PrintString` (`KismetStringLibrary.Concat_StrStr` "[NoCollision] " (`KismetSystemLibrary.GetDisplayName` _array_element))))))

(event `self.GrabComponent.OnDropped`
  ; OnGrabbed
  (for _array_element (`/Game/BluePrints/PuzzleLevel/Tooth/BP_ToothPieceBase.AttachedPieceArray` (`self.RootActor`))
    (`PrimitiveComponent.SetCollisionEnabled` (`/Game/BluePrints/PuzzleLevel/Tooth/BP_ToothPieceBase.ToothCell` _array_element) "QueryAndPhysics")
    (`KismetSystemLibrary.PrintString` (`KismetStringLibrary.Concat_StrStr` "[CollisionEnabled] " (`KismetSystemLibrary.GetDisplayName` _array_element)))))

(fn `UserConstructionScript`)