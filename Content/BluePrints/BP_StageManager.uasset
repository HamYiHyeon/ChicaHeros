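; Stage manager for a VR cavity game that runs a bacteria combat stage from fade-in to win or loss.
; BeginPlay shuffles tooth spawn points, marks the chosen ones with decay material and smoke, and maps GameInstance StageInfo to enemy classes and count.
; Player hits update the HP bar and trigger glitch effects.
; Death, timeout or clear records the result, pays gold on clear, and glitch-fades back to the waiting room.
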(event `self.OnPlayerAttackedBP`
  (params (Damage :type "Float (single-precision)"))
  ; Hit
  (`GameplayStatics.PlaySoundAtLocation` "/Game/Sound/metal-hit-5-193273.metal-hit-5-193273" (`self.K2_GetActorLocation` (`self.PlayerPawn`)) (struct) 1.0 1.0 0.0 null null null null)
  (if (not (`self.CastHPBar`))
    (bind _asvr_cavity_player_pawn (cast `/Game/BluePrints/StageLevel/VR_CavityPlayerPawn` (`self.PlayerPawn`)))
    (bind _aswbp_healthbar (cast `/Game/UI/Widgets/Stage/WBP_healthbar` (`WidgetComponent.GetUserWidgetObject` (`/Game/BluePrints/StageLevel/VR_CavityPlayerPawn.HPBar` _asvr_cavity_player_pawn)))
      (:`then`
        (`KismetSystemLibrary.PrintString` "cast hpbar success")
        (set `self.CastHPBar` true)
        (bind _output_get (set `self.PlayerHp` (- (`self.PlayerHp`) Damage) :!label _label))
        (`/Game/UI/Widgets/Stage/WBP_healthbar.UpdateHP` _aswbp_healthbar (/ _output_get (`self.PlayerMaxHP`)))
        (`/Game/BluePrints/BP_Glitch.HitGlitch` (`self.BP_Glitch`))
        (if (<= (`self.PlayerHp`) 0.0)
          (bind _asbp_game_instance (cast `/Game/BluePrints/BP_GameInstance` (`GameplayStatics.GetGameInstance`)))
          (set `/Game/BluePrints/BP_GameInstance.bStageCleared` false _asbp_game_instance)
          (`self.SceneChange`)))
      (:`CastFailed`
        (`KismetSystemLibrary.PrintString` "cast hpbar fail")))
    (else
      (goto _label))))

(event `self.ReceiveBeginPlay`
  (bind _spawnpointarray (`self.SpawnPointArray`))
  (bind _enemyarray (`self.Enemyarray`))
  (bind _enemy (`self.Enemy`))
  (bind _stagenum (`self.StageNum`))
  (`|ExecutionSequence`
    (:`then_0`
      (`/Game/BluePrints/BP_Glitch.Glitch` (`self.BP_Glitch`))
      (`self.FadeIn`)
      (set `self.PlayerHp` (`self.PlayerMaxHP`)))
    (:`then_1`
      (`KismetArrayLibrary.Array_Shuffle` _spawnpointarray)
      (for _index (range (+ (`self.SpawnPointNum`) 1))
        (bind _output (`|GetArrayItem` _spawnpointarray _index))
        (bind _returnvalue (`SceneComponent.K2_GetComponentLocation` (`/Game/BluePrints/StageLevel/BP_SpawnPoint.SpawnPointLocation` _output)))
        (`KismetArrayLibrary.Array_Add` (`self.SpawnPoint`) _returnvalue)
        (bind _returnvalue_2 (`PrimitiveComponent.CreateDynamicMaterialInstance` (`/Game/BluePrints/StageLevel/BP_SpawnPoint.Tooth` _output) 0 "/Game/BluePrints/StageLevel/StageLevelMat/M_StageMaster_Inst.M_StageMaster_Inst" "None"))
        (`MaterialInstanceDynamic.SetScalarParameterValueByInfo` _returnvalue_2 (make `MaterialParameterInfo` "ScalarOpacity" "LayerParameter" 1) 1.0)
        (`NiagaraFunctionLibrary.SpawnSystemAtLocation` "/Game/Niagara/NS_Smoke.NS_Smoke" _returnvalue (struct) (1.0 1.0 1.0) false)))
    (:`then_2`
      (bind _asbp_game_instance (cast `/Game/BluePrints/BP_GameInstance` (`GameplayStatics.GetGameInstance`)))
      (for _index_2 (range 2) :!label _label_2
        (bind _stageinfo (`/Game/BluePrints/BP_GameInstance.StageInfo` _asbp_game_instance))
        (`KismetArrayLibrary.Array_Set` _enemyarray _index_2 (`|GetArrayItem` _stageinfo (+ _index_2 (* _stagenum 3)))))
      (for (_array_element _array_index) _enemyarray
        (if (< (`KismetArrayLibrary.Array_Length` _enemy) 2)
          (bind _value (`BlueprintMapLibrary.Map_Find` (`self.BacteriaClassMap`) _array_element))
          (`KismetArrayLibrary.Array_Add` _enemy _value)
          (else
            (`KismetArrayLibrary.Array_Set` _enemy _array_index _value))))
      (set `self.EnemyCount` (`|GetArrayItem` _stageinfo (+ (* _stagenum 3) 2))))))

(event `self.MonsterInfo`
  (goto _label_2))

(event `self.GameClear`
  (bind _asbp_game_instance (cast `/Game/BluePrints/BP_GameInstance` (`GameplayStatics.GetGameInstance`)))
  (set `/Game/BluePrints/BP_GameInstance.bStageCleared` true _asbp_game_instance)
  (set `/Game/BluePrints/BP_GameInstance.Gold` (+ (`/Game/BluePrints/BP_GameInstance.Reward` _asbp_game_instance) (`/Game/BluePrints/BP_GameInstance.Gold` _asbp_game_instance)) _asbp_game_instance)
  (`self.SceneChange`))

(event `self.TimeOver`
  (set `/Game/BluePrints/BP_GameInstance.bStageCleared` false (stale `self.GameClear` _asbp_game_instance))
  (`self.SceneChange`))

(event `SceneChange`
  ; SceneChange
  (`self.GameStop`)
  (`/Game/BluePrints/BP_Glitch.GlitchOut` (`self.BP_Glitch`))
  (`KismetSystemLibrary.Delay` 0.7)
  (`self.FadeOut`)
  (`KismetSystemLibrary.Delay` 0.3)
  (`GameplayStatics.OpenLevel` "WatingRoom"))

(event `GameStop`
  ; GameStop
  (`self.TickDisable`)
  (`KismetSystemLibrary.K2_ClearTimer` null "SpawnTimerHandle"))

(event `FadeIn`
  ; FadeIn
  (`PlayerCameraManager.StartCameraFade` :`self` (`PlayerController.PlayerCameraManager` (`GameplayStatics.GetPlayerController` 0)) :`FromAlpha` 1.0 :`Duration` 2.0))

(event `FadeOut`
  ; FadeOut
  (`PlayerCameraManager.StartCameraFade` :`self` (`PlayerController.PlayerCameraManager` (`GameplayStatics.GetPlayerController` 0)) :`ToAlpha` 1.0 :`Duration` 0.3 :`bHoldWhenFinished` true))

(fn `UserConstructionScript`)