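; VR level selector menu actor that hosts the VRLevelSelectorMaster widget for pointer-based selection.
; On BeginPlay it caches the VR_PlayerPawn, disables that pawn's tick, enables input and adds the IMC_Menu mapping context.
; Left and right interact actions press and release a simulated left mouse button on the pawn's matching WidgetInteraction component.
; Tick calls RotateMainMenu, whose interpolated camera-follow logic is disconnected, so the menu does not move.
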(event `self.ReceiveBeginPlay`
  (bind _returnvalue (`GameplayStatics.GetPlayerController` 0))
  (bind _asvr_player_pawn (cast `/Game/GameProject_Player/VR_PlayerPawn` (`GameplayStatics.GetPlayerPawn` 0)))
  (bind _output_get (set `self.VRPlayerPawn` _asvr_player_pawn))
  (`self.SetActorTickEnabled` _output_get false)
  (`self.EnableInput` _returnvalue)
  (`EnhancedInputSubsystemInterface.AddMappingContext` (pcsubsystem `EnhancedInputLocalPlayerSubsystem` _returnvalue) "/Game/VRTemplate/Input/IMC_Menu.IMC_Menu" 1 (struct))
  (bind _asvrlevel_selector_master (cast `/Game/BluePrints/VRLevelSelectorMaster` (`WidgetComponent.GetWidget` (`self.Widget`)))))

(event `self.ReceiveTick`
  (params (DeltaSeconds :type "Float (single-precision)"))
  (`self.Rotate Main Menu` DeltaSeconds))

(event `EnhancedInput|/Game/VRTemplate/Input/Actions/IA_Menu_Interact_Left_Pressed`
  (params (ActionValue :type Boolean) (ElapsedSeconds :type "Float (double-precision)") (TriggeredSeconds :type "Float (double-precision)") (InputAction :type "InputAction Object Reference" :default "/Game/VRTemplate/Input/Actions/IA_Menu_Interact_Left_Pressed.IA_Menu_Interact_Left_Pressed"))
  (bind _widgetinteractionleft (`/Game/GameProject_Player/VR_PlayerPawn.WidgetInteractionLeft` (`self.VRPlayerPawn`)))
  (:`Started`
    (`WidgetInteractionComponent.PressPointerKey` _widgetinteractionleft "LeftMouseButton"))
  (:`Canceled`
    (`WidgetInteractionComponent.ReleasePointerKey` _widgetinteractionleft "LeftMouseButton" :!label _label))
  (:`Completed`
    (goto _label)))

(event `EnhancedInput|/Game/VRTemplate/Input/Actions/IA_Menu_Interact_Right_Pressed`
  (params (ActionValue :type Boolean) (ElapsedSeconds :type "Float (double-precision)") (TriggeredSeconds :type "Float (double-precision)") (InputAction :type "InputAction Object Reference" :default "/Game/VRTemplate/Input/Actions/IA_Menu_Interact_Right_Pressed.IA_Menu_Interact_Right_Pressed"))
  (bind _widgetinteractionright (`/Game/GameProject_Player/VR_PlayerPawn.WidgetInteractionRight` (`self.VRPlayerPawn`)))
  (:`Started`
    (`WidgetInteractionComponent.PressPointerKey` _widgetinteractionright "LeftMouseButton"))
  (:`Canceled`
    (`WidgetInteractionComponent.ReleasePointerKey` _widgetinteractionright "LeftMouseButton" :!label _label_2))
  (:`Completed`
    (goto _label_2)))

(fn `Rotate Main Menu`
  (params (DeltaTime :type "Float (double-precision)")))

(fn `UserConstructionScript`)