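; BP_Gemella is a bacteria actor in a VR cavity game that awards points to the player when destroyed.
; Its capsule's begin overlap passes the other actor to HitBac, whose logic is not defined in this graph.
; On destruction it casts its PlayerPawn reference to VR_CavityPlayerPawn and adds its own Point value to the pawn's total.
; The end-overlap check for a Pistol tag has no effect.
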(event `self.Capsule.OnComponentBeginOverlap`
  (params (OverlappedComponent :type "PrimitiveComponent Object Reference") (OtherActor :type "Actor Object Reference") (OtherComp :type "PrimitiveComponent Object Reference") (OtherBodyIndex :type Integer) (bFromSweep :type Boolean) (SweepResult :type "HitResult Structure (by ref)"))
  (`self.HitBac` OtherActor))

(event `self.Capsule.OnComponentEndOverlap`
  (params (OverlappedComponent :type "PrimitiveComponent Object Reference") (OtherActor :type "Actor Object Reference") (OtherComp :type "PrimitiveComponent Object Reference") (OtherBodyIndex :type Integer))
  (if (`self.ActorHasTag` OtherActor "Pistol")
    _))

(event `self.ReceiveDestroyed`
  (bind _asvr_cavity_player_pawn (cast `/Game/BluePrints/StageLevel/VR_CavityPlayerPawn` (`self.PlayerPawn`)))
  (set `/Game/BluePrints/StageLevel/VR_CavityPlayerPawn.Point` (+ (`/Game/BluePrints/StageLevel/VR_CavityPlayerPawn.Point` _asvr_cavity_player_pawn) (`self.Point`)) _asvr_cavity_player_pawn))

(fn `UserConstructionScript`)