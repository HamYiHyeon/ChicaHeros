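; BP_NanoRobot is a robot character that reflects the last stage result through its animation.
; On BeginPlay it reads BP_GameInstance, setting StageCleared to a win or loss value, or only flagging GameStart if the game has not yet started.
; It then passes that value and a random dance index to ABP_NanoRobot on the LowPBot0101 mesh.
; Tick and ClearResult are empty.
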(event `self.ReceiveBeginPlay`
  (`|ExecutionSequence`
    (:`then_0`
      (bind _asbp_game_instance (cast `/Game/BluePrints/BP_GameInstance` (`GameplayStatics.GetGameInstance`)))
      (if (`/Game/BluePrints/BP_GameInstance.GameStart` _asbp_game_instance)
        (if (`/Game/BluePrints/BP_GameInstance.bStageCleared` _asbp_game_instance)
          (set `self.StageCleared` 1)
          (else
            (set `self.StageCleared` -1)))
        (else
          (set `/Game/BluePrints/BP_GameInstance.GameStart` true _asbp_game_instance))))
    (:`then_1`
      (bind _asabp_nano_robot (cast `/Game/BluePrints/ABP_NanoRobot` (`SkeletalMeshComponent.GetAnimInstance` (`self.Low_P_Bot_0101`))))
      (set `/Game/BluePrints/ABP_NanoRobot.ABPStageCleared` (`self.StageCleared`) _asabp_nano_robot)
      (set `/Game/BluePrints/ABP_NanoRobot.ABPDanceIndex` (`KismetMathLibrary.RandomIntegerInRange` 0 2) _asabp_nano_robot))))

(event `self.ReceiveTick`
  (params (DeltaSeconds :type "Float (single-precision)")))

(event `self.ClearResult`)

(fn `UserConstructionScript`)