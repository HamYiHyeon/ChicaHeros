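; BP_ToothBase is a tooth actor that can start dirty and be cleaned by a water gun.
; On BeginPlay a random boolean picks either a black dirty material, setting IsDirty, or the normal tooth material.
; When the static mesh overlaps a WaterGun1, CleanTooth raises a clamped progress value, which completes in a single hit, then restores the tooth material and clears IsDirty.
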(event `self.StaticMesh.OnComponentBeginOverlap`
  (params (OverlappedComponent :type "PrimitiveComponent Object Reference") (OtherActor :type "Actor Object Reference") (OtherComp :type "PrimitiveComponent Object Reference") (OtherBodyIndex :type Integer) (bFromSweep :type Boolean) (SweepResult :type "HitResult Structure (by ref)"))
  (cast `/Game/GameProject_Player/Asset/WaterGun1` OtherActor
    (:`then`
      (`self.CleanTooth`))
    (:`CastFailed`
      _))
  (`KismetSystemLibrary.PrintString` "clean"))

(event `self.ReceiveBeginPlay`
  (bind _staticmesh (`self.StaticMesh`))
  (if (`KismetMathLibrary.RandomBool`)
    (`PrimitiveComponent.SetMaterial` _staticmesh 0 "/Engine/EngineDebugMaterials/BlackUnlitMaterial.BlackUnlitMaterial")
    (set `self.IsDirty` true)
    (else
      (`PrimitiveComponent.SetMaterial` _staticmesh 0 "/Game/Asset/denture/dente.dente"))))

(fn `CleanTooth`
  (if (`self.IsDirty`)
    (set `self.CleanProgress` (`KismetMathLibrary.FClamp` (+ (`self.CleanProgress`) 1.0)))
    (if (>= (`self.CleanProgress`) 1.0)
      (`PrimitiveComponent.SetMaterial` (`self.StaticMesh`) 0 "/Game/Asset/denture/dente.dente")
      (set `self.IsDirty` false))))

(fn `UserConstructionScript`)