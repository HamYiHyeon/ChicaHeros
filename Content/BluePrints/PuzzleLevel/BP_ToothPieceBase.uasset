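; Base Blueprint for a grabbable tooth piece in a puzzle that snaps to other pieces to rebuild a tooth.
; While its sphere overlaps another piece, Tick allows attachment if each rotation axis differs by at most 15 degrees.
; Dropping then snaps it to that piece and merges both groups' shared arrays, flagging the PuzzleManager clear at six pieces.
; Grabbing re-parents the group to the held piece and disables the other members' collision.
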(event `self.ReceiveBeginPlay`
  ; BeginPlay
  (`KismetArrayLibrary.Array_Add` (`self.AttachedPieceArray`) self))

(event `self.Sphere.OnComponentEndOverlap`
  (params (OverlappedComponent :type "PrimitiveComponent Object Reference") (OtherActor :type "Actor Object Reference") (OtherComp :type "PrimitiveComponent Object Reference") (OtherBodyIndex :type Integer))
  ; AbleAttach
  (set `self.bOverlapping` false)
  (`KismetSystemLibrary.PrintString` "overlap end"))

(event `self.Sphere.OnComponentBeginOverlap`
  (params (OverlappedComponent :type "PrimitiveComponent Object Reference") (OtherActor :type "Actor Object Reference") (OtherComp :type "PrimitiveComponent Object Reference") (OtherBodyIndex :type Integer) (bFromSweep :type Boolean) (SweepResult :type "HitResult Structure (by ref)"))
  ; AbleAttach
  (bind _asbp_tooth_piece_base (cast `/Game/BluePrints/PuzzleLevel/BP_ToothPieceBase` OtherActor))
  (bind _output_get (set `self.OtherToothPiece` _asbp_tooth_piece_base))
  (set `self.bOverlapping` true)
  (`KismetSystemLibrary.PrintString` (`KismetStringLibrary.Concat_StrStr` "overlap: " (`KismetSystemLibrary.GetDisplayName` _output_get))))

(event `self.ReceiveTick`
  (params (DeltaSeconds :type "Float (single-precision)"))
  (bind _returnvalue (`KismetMathLibrary.Abs` (- (.yaw (`SceneComponent.K2_GetComponentRotation` (`/Game/BluePrints/PuzzleLevel/BP_ToothPieceBase.GrabComponent` (`self.OtherToothPiece`)))) (.yaw (`SceneComponent.K2_GetComponentRotation` (`self.GrabComponent`))))))
  (bind _returnvalue_2 (`KismetMathLibrary.Abs` (- (.roll (`SceneComponent.K2_GetComponentRotation` (`/Game/BluePrints/PuzzleLevel/BP_ToothPieceBase.GrabComponent` (`self.OtherToothPiece`)))) (.roll (`SceneComponent.K2_GetComponentRotation` (`self.GrabComponent`))))))
  (bind _returnvalue_3 (`KismetMathLibrary.Abs` (- (.pitch (`SceneComponent.K2_GetComponentRotation` (`/Game/BluePrints/PuzzleLevel/BP_ToothPieceBase.GrabComponent` (`self.OtherToothPiece`)))) (.pitch (`SceneComponent.K2_GetComponentRotation` (`self.GrabComponent`))))))
  ; AbleAttach
  (if (`self.bOverlapping`)
    (`KismetSystemLibrary.PrintString` (`KismetStringLibrary.Concat_StrStr` "Rotation(" (`KismetStringLibrary.Conv_DoubleToString` _returnvalue_2) ", " (`KismetStringLibrary.Conv_DoubleToString` _returnvalue_3) ", " (`KismetStringLibrary.Conv_DoubleToString` _returnvalue) ")"))
    (if (and (<= _returnvalue_2 15.0) (<= _returnvalue_3 15.0) (<= _returnvalue 15.0))
      (set `self.bAbleAttach` true)
      (`KismetSystemLibrary.PrintString` "AbleAttach")
      (else
        (set `self.bAbleAttach` false :!label _label)))
    (else
      (goto _label))))

(event `Attach`
  (bind _temparray (`self.TempArray`))
  ; AttachComponentToComponent
  (`SceneComponent.K2_AttachToComponent` (`self.ToothCell`) (`/Game/BluePrints/PuzzleLevel/BP_ToothPieceBase.ToothCell` (`self.OtherToothPiece`)) "None" "SnapToTarget" "SnapToTarget" "KeepWorld" true)
  (`PrimitiveComponent.SetCollisionEnabled` (`self.Sphere`) "NoCollision")
  (set `self.TempArray` (`self.AttachedPieceArray`))
  (for _array_element (`/Game/BluePrints/PuzzleLevel/BP_ToothPieceBase.AttachedPieceArray` (`self.OtherToothPiece`))
    (`KismetArrayLibrary.Array_AddUnique` _temparray _array_element))
  (for _array_element_2 _temparray
    (bind _output_get (set `/Game/BluePrints/PuzzleLevel/BP_ToothPieceBase.AttachedPieceArray` _temparray _array_element_2)))
  (`KismetSystemLibrary.PrintString` (`KismetStringLibrary.Concat_StrStr` "Attachto: " (`KismetSystemLibrary.GetDisplayName` (`self.OtherToothPiece`))))
  (if (>= (`KismetArrayLibrary.Array_Length` _output_get) 6)
    (set `/Game/BluePrints/PuzzleLevel/BP_PuzzleManager.IsClear?` true (`self.PuzzleManager`))))

(event `self.GrabComponent.OnGrabbed`
  ; OnGrabbed
  (`PrimitiveComponent.SetCollisionEnabled` (`self.Sphere`) "QueryOnly")
  (for _array_element (`self.AttachedPieceArray`)
    (`KismetSystemLibrary.PrintString` (`KismetStringLibrary.Concat_StrStr` "Reattach: " (`KismetSystemLibrary.GetDisplayName` _array_element)))
    (if (!= _array_element self)
      (bind _toothcell (`/Game/BluePrints/PuzzleLevel/BP_ToothPieceBase.ToothCell` _array_element))
      (`SceneComponent.K2_AttachToComponent` _toothcell (`self.ToothCell`) "None" "SnapToTarget" "SnapToTarget" "KeepWorld" true)
      (`PrimitiveComponent.SetCollisionEnabled` _toothcell "NoCollision")
      (`PrimitiveComponent.SetCollisionEnabled` (`/Game/BluePrints/PuzzleLevel/BP_ToothPieceBase.Sphere` _array_element) "NoCollision")
      (`KismetSystemLibrary.PrintString` (`KismetStringLibrary.Concat_StrStr` "[NoCollision] " (`KismetSystemLibrary.GetDisplayName` _array_element)))))
  (`self.Debug`))

(event `self.GrabComponent.OnDropped`
  ; OnDropped
  (`KismetSystemLibrary.PrintString` (`KismetStringLibrary.Concat_StrStr` "Dropped: " (`KismetSystemLibrary.GetDisplayName` self)))
  (if (`self.bAbleAttach`)
    (`self.Attach`)
    (`PrimitiveComponent.SetCollisionEnabled` (`self.ToothCell`) "NoCollision")
    (else
      (for _array_element (`self.AttachedPieceArray`)
        (`PrimitiveComponent.SetCollisionEnabled` (`/Game/BluePrints/PuzzleLevel/BP_ToothPieceBase.ToothCell` _array_element) "QueryAndPhysics")
        (`KismetSystemLibrary.PrintString` (`KismetStringLibrary.Concat_StrStr` "[CollisionEnabled] " (`KismetSystemLibrary.GetDisplayName` _array_element)))))))

(event `Debug`
  (`KismetSystemLibrary.PrintString` (`KismetStringLibrary.Concat_StrStr` "Grabbed: AbleAttach(" (`KismetStringLibrary.Conv_BoolToString` (`self.bAbleAttach`)) ") / Overlapping(" (`KismetStringLibrary.Conv_BoolToString` (`self.bOverlapping`)) ") / SphereCollision(" (`|GetEnumeratorNameAsString` (`PrimitiveComponent.GetCollisionEnabled` (`self.Sphere`))))))

(fn `UserConstructionScript`)