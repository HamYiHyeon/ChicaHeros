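; BP_Tooth is a set of 32 tooth meshes that can start dirty and be cleaned.
; On BeginPlay, each tooth randomly gets either a black unlit dirty material or the clean Dente material.
; CleanTooth, when IsDirty is set, fills the clamped CleanProgress in one call and restores Dente on all teeth at once.
; It then sets IsDirty to true again, so the dirty flag is never cleared here.
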(event `self.ReceiveBeginPlay`
  (for _array_element (`|MakeArray` (`self.ToothHead_032`) (`self.ToothHead_031`) (`self.ToothHead_030`) (`self.ToothHead_029`) (`self.ToothHead_028`) (`self.ToothHead_027`) (`self.ToothHead_026`) (`self.ToothHead_025`) (`self.ToothHead_024`) (`self.ToothHead_023`) (`self.ToothHead_022`) (`self.ToothHead_021`) (`self.ToothHead_020`) (`self.ToothHead_019`) (`self.ToothHead_018`) (`self.ToothHead_017`) (`self.ToothHead_016`) (`self.ToothHead_015`) (`self.ToothHead_014`) (`self.ToothHead_013`) (`self.ToothHead_012`) (`self.ToothHead_011`) (`self.ToothHead_010`) (`self.ToothHead_009`) (`self.ToothHead_008`) (`self.ToothHead_007`) (`self.ToothHead_006`) (`self.ToothHead_005`) (`self.ToothHead_004`) (`self.ToothHead_003`) (`self.ToothHead_002`) (`self.ToothHead_001`))
    (if (`KismetMathLibrary.RandomBool`)
      (`PrimitiveComponent.SetMaterial` _array_element 0 "/Engine/EngineDebugMaterials/BlackUnlitMaterial.BlackUnlitMaterial")
      (else
        (`PrimitiveComponent.SetMaterial` _array_element 0 "/Game/Asset/denture/dente.dente")))))

(fn `CleanTooth`
  (if (`self.IsDirty`)
    (set `self.CleanProgress` (`KismetMathLibrary.FClamp` (+ (`self.CleanProgress`) 1.0) 0.0 1.0))
    (if (>= (`self.CleanProgress`) 1.0)
      (`PrimitiveComponent.SetMaterial` (`|MakeArray` (`self.ToothHead_032`) (`self.ToothHead_031`) (`self.ToothHead_030`) (`self.ToothHead_029`) (`self.ToothHead_028`) (`self.ToothHead_027`) (`self.ToothHead_026`) (`self.ToothHead_025`) (`self.ToothHead_024`) (`self.ToothHead_023`) (`self.ToothHead_022`) (`self.ToothHead_021`) (`self.ToothHead_020`) (`self.ToothHead_019`) (`self.ToothHead_018`) (`self.ToothHead_017`) (`self.ToothHead_016`) (`self.ToothHead_015`) (`self.ToothHead_014`) (`self.ToothHead_013`) (`self.ToothHead_012`) (`self.ToothHead_011`) (`self.ToothHead_010`) (`self.ToothHead_009`) (`self.ToothHead_008`) (`self.ToothHead_007`) (`self.ToothHead_006`) (`self.ToothHead_005`) (`self.ToothHead_004`) (`self.ToothHead_003`) (`self.ToothHead_002`) (`self.ToothHead_001`)) 0 "/Game/Asset/denture/dente.dente")
      (set `self.IsDirty` true))))

(fn `UserConstructionScript`)