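; Robot trophy actor, apparently for the game's ending, that glides to a new position shortly after play begins.
; BeginPlay stores the start location, waits, then runs Timeline_FloatUp to lerp the actor along negative world X, despite the timeline's name.
; The same alpha blends rotation through X vectors, but the StartRotation and TargetRotation setters are unconnected, so both keep their defaults.
; The trailing local rotation adds zero.
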(event `self.ReceiveBeginPlay`
  (bind _output_get (set `self.Start Location` (`self.K2_GetActorLocation`)))
  (set `self.Target Location` (+ _output_get (-200.0 0.0 0.0)))
  (`KismetSystemLibrary.Delay` 2.5)
  (bind (_direction _fadeprogress) (`Timeline|Timeline_FloatUp` :`NewTime` 5.0)
    (:`Update`
      (`self.K2_SetActorRotation` (`KismetMathLibrary.Conv_VectorToRotator` (`KismetMathLibrary.VLerp` (`KismetMathLibrary.Conv_RotatorToVector` (`self.Start Rotation`)) (`KismetMathLibrary.Conv_RotatorToVector` (`self.Target Rotation`)) _fadeprogress)))
      (`self.K2_SetActorLocation` (`KismetMathLibrary.VLerp` (`self.Start Location`) (`self.Target Location`) _fadeprogress))
      (`self.K2_AddActorLocalRotation` (struct)))))

(fn `UserConstructionScript`)